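; Test game mode Blueprint that checks player login through a ControllerLogin component.
; On PostLogin, when the TestLogin flag is set, it looks up that component and prints "Already Logged In" if login is already complete.
; Otherwise it binds LoginFinished to the component's OnLogin event, which prints the controller's display name with a "Logged In" message.
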(event `LoginFinished`
  (params (Controller :type "PlayerController Object Reference"))
  ;[1 1 1] Test Login
  (`KismetSystemLibrary.PrintString` (`KismetStringLibrary.Concat_StrStr` (`KismetSystemLibrary.GetDisplayName` Controller) " Logged In")))

(event `self.K2_PostLogin`
  (params (NewPlayer :type "PlayerController Object Reference"))
  (bind _returnvalue (`self.GetComponentByClass` "/Script/PlebComponents.ControllerLogin"))
  (`|ExecutionSequence`
    (:`then_0`
      ;[1 1 1] Test Login
      (if (`self.TestLogin`)
        (if (!= _returnvalue null)
          (if (`ControllerLogin.IsLoggedIn` _returnvalue)
            (`KismetSystemLibrary.PrintString` "Already Logged In")
            (else
              (add `ControllerLogin.OnLogin` _returnvalue (delegate `LoginFinished`)))))))))

(fn `UserConstructionScript`)