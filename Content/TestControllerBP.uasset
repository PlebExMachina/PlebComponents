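; Test player controller that triggers character selection from number keys.
; Keys 1 and 2 check the game mode, then pass ThirdPersonCharacter or the default Pawn to CharacterSelectCompanion and print the choice.
; Key 3 skips that check and calls ChooseCharacter directly on the GameState's CharacterSelect component, passing itself as the player with ThirdPersonCharacter.
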(event `Key|One`
  (params (Key :type "Key Structure"))
  (:`Pressed`
    (if (== (`GameplayStatics.GetGameMode`) null)
      (`CharacterSelectCompanion.ChooseCharacter` (`self.CharacterSelectCompanion`) "/Game/ThirdPersonCPP/Blueprints/ThirdPersonCharacter.ThirdPersonCharacter_C")
      (`KismetSystemLibrary.PrintString` "TPC CHOSEN"))))

(event `Key|Two`
  (params (Key :type "Key Structure"))
  (:`Pressed`
    (if (== (`GameplayStatics.GetGameMode`) null)
      (`CharacterSelectCompanion.ChooseCharacter` (`self.CharacterSelectCompanion`) "/Script/Engine.Pawn")
      (`KismetSystemLibrary.PrintString` "DEFAULT PAWN CHOSEN"))))

(event `Key|Three`
  (params (Key :type "Key Structure"))
  (:`Pressed`
    (`CharacterSelect.ChooseCharacter` (`self.GetComponentByClass` (`GameplayStatics.GetGameState`) "/Script/PlebComponents.CharacterSelect") self "/Game/ThirdPersonCPP/Blueprints/ThirdPersonCharacter.ThirdPersonCharacter_C")))

(fn `UserConstructionScript`)